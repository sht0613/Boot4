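; BP_Slash is a slash skill actor that deals a one-shot area attack around its Character.
; On BeginPlay it snaps onto the character's mesh, then applies radial damage at its location, ignoring the character and crediting its controller as instigator.
; The Attack particle system's finish event drives cleanup, destroying the actor when the effect ends.
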(event EventBeginPlay
  (EventDispatchers|BindEventtoOnSystemFinished (Variables|Default|GetAttack) (EventDispatchers|CreateEvent :!event EventFinishAttack))
  (Transformation|AttachComponentToComponent (Variables|/Script/Engine.Character|GetMesh (Variables|Default|GetCharacter)) "None" "SnapToTarget" "SnapToTarget" "KeepWorld" true)
  (Game|Damage|ApplyRadialDamage 5e+01 (Transformation|GetActorLocation) 5e+02 0 (Utilities|Array|MakeArray (Variables|Default|GetCharacter)) self (Pawn|GetController (Variables|Default|GetCharacter)) false "ECC_Visibility"))

(fn ConstructionScript)

(fn EventFinishAttack
  (params (PSystem :type Niagara%20Component%20Object%20Reference))
  (Actor|DestroyActor))