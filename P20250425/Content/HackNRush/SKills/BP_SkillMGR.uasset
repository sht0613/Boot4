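; BP_SkillMGR is a skill manager that automatically casts its owner's skills whenever their cooldowns elapse.
; AddSkill looks up a row in DT_SKill and stores it with its timer preset to the cooldown, so it fires on the next update.
; Each Tick advances every timer; when one passes its cooldown, it spawns that skill's actor class at the owner's transform, passing the owning Character, then resets the timer.
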(event EventTick
  (params (DeltaSeconds :type Float%20%28single-precision%29))
  (CallFunction|UpdateSkills DeltaSeconds))

(fn AddSkill
  (params (SkillRowName :type Name))
  (bind _returnvalue (Utilities|GetDataTableRow "/Game/HackNRush/SKills/DT_SKill.DT_SKill" SkillRowName)
    (:then
      (Utilities|Array|Add (Variables|Default|GetSkills) (Utilities|Struct|MakeST_CurSkill _returnvalue (.CoolTime (Utilities|Struct|BreakST_Skill _returnvalue)))))))

(fn UpdateSkills
  (params (DeltaSec :type Float%20%28double-precision%29))
  (for (_ _array_index) (Variables|Default|GetSkills)
    (CallFunction|UpdateSkillCollTime (Utilities|Array|Get(acopy) (Variables|Default|GetSkills) _array_index) DeltaSec)))

(fn DoUseSKill
  (params (CurSkill :type ST%20Cur%20Skill%20Structure))
  (bind _returnvalue (Components|GetOwner))
  (bind _ascharacter (Utilities|Casting|CastToCharacter _returnvalue))
  (Game|SpawnActorfromClass (.skillclass (.SkillData (Utilities|Struct|BreakST_CurSkill CurSkill))) (Transformation|GetActorTransform _returnvalue) "Undefined" "MultiplyWithRoot" 0 _ascharacter 0))

(fn UpdateSkillCollTime
  (params (CurSkill :type ST%20Cur%20Skill%20Structure%20%28by%20ref%29) (DeltaSecond :type Float%20%28double-precision%29))
  (bind _structout (Utilities|Struct|SetmembersinST_CurSkill CurSkill (+ (.CurCoolTime (Utilities|Struct|BreakST_CurSkill CurSkill)) DeltaSecond)))
  (if (> (.CurCoolTime (Utilities|Struct|BreakST_CurSkill _structout)) (.cooltime (.SkillData (Utilities|Struct|BreakST_CurSkill _structout))))
    (CallFunction|DoUseSKill _structout)
    (Utilities|Struct|SetmembersinST_CurSkill _structout 0.0)))