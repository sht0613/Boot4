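; BP_MonStatComponent is a stat component for monsters that tracks current HP and death state.
; SetMonStat loads a named row from DT_Monster, starts current HP at the row's MaxHP and broadcasts the new stats.
; AddDamage skips dead monsters, otherwise subtracts damage, broadcasts the HP update and fires the death dispatcher when HP reaches zero or below.
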(fn SetMonStat
  (params (RowName :type Name))
  (bind _returnvalue (Utilities|GetDataTableRow "/Game/HackNRush/Monster/DT_Monster.DT_Monster" RowName)
    (:then
      (bind _output_get (Variables|Default|SetCurMonStat (Utilities|Struct|MakeST_CurMonster _returnvalue (.MaxHP (Utilities|Struct|BreakST_Monster _returnvalue)))))
      (Default|CallNewEventDispatcherMonStat _output_get))))

(fn AddDamage
  (params (Damage :type Float%20%28double-precision%29))
  (bind _curmonstat (Variables|Default|GetCurMonStat))
  (if (not (CallFunction|IsDeath))
    (bind _structout (Utilities|Struct|SetmembersinST_CurMonster (Variables|Default|GetCurMonStat) (- (.curhp (Variables|Default|GetCurMonStat)) Damage)))
    (Default|CallNewEventDispatcherUpdateHP (.curhp _curmonstat) (.maxhp (.mondata _curmonstat)))
    (if (<= (.CurHP (Utilities|Struct|BreakST_CurMonster _structout)) 0.0)
      (Default|CallNewEventDispatcherDeath (Variables|Default|GetCurMonStat)))))

(fn IsDeath
  (return (<= (.curhp (Variables|Default|GetCurMonStat)) 0.0)))