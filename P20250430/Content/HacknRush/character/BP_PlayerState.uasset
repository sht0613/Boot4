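; BP_PlayerState holds a player's health and three Red, Green and Blue counters.
; AddDamage subtracts HP unless already dead, and fires the death dispatcher when HP reaches zero or below.
; AddHeal clamps to a fixed 0–100 range rather than MaxHP; both health functions broadcast UpdateHP, which feeds the NameTag.
; Each color Add function increments its counter and broadcasts it through its own event dispatcher.
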(event EventBeginPlay)

(event EventTick
  (params (DeltaSeconds :type Float%20%28single-precision%29)))

(fn ConstructionScript)

(fn IsDeath
  (return (<= (Variables|Default|GetCurHP) 0.0)))

(fn AddDamage
  (params (Damage :type Float%20%28double-precision%29))
  (if (not (CallFunction|IsDeath))
    (bind _output_get (Variables|Default|SetCurHP (- (Variables|Default|GetCurHP) Damage)))
    (Default|CallEventDispatcherUpdateHP _output_get (Variables|Default|GetMaxHP))
    (if (<= (Variables|Default|GetCurHP) 0.0)
      (Default|CallEventDispatcherDeath))))

(fn AddHeal
  (params (Heal :type Float%20%28double-precision%29))
  (bind _output_get (Variables|Default|SetCurHP (Math|Float|Clamp(Float) (+ Heal (Variables|Default|GetCurHP)) 0.0 1e+02)))
  ;[0.15 0.15 0.15 0.5] NameTag에 HP 업뎃 정보 전달
  (Default|CallEventDispatcherUpdateHP _output_get (Variables|Default|GetMaxHP)))

(fn AddRed
  (bind _output_get (Variables|Default|SetRed (+ (Variables|Default|GetRed) 1)))
  (Default|CallEventDispatcherRed _output_get))

(fn AddGreen
  (bind _output_get (Variables|Default|SetGreen (+ (Variables|Default|GetGreen) 1)))
  (Default|CallEventDispatcherGreen _output_get))

(fn AddBlue
  (bind _output_get (Variables|Default|SetBlue (+ (Variables|Default|GetBlue) 1)))
  (Default|CallEventDispatcherBlue _output_get))