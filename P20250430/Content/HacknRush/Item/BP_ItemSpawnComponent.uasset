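; BP_ItemSpawnComponent periodically spawns random item actors around its owning actor.
; A looping timer started on BeginPlay calls DoSpawn every few seconds.
; DoSpawn picks a random DT_Item row and spawns its ItemClass at a random navigable point near the owner.
; The SpawnCount limit logic is disconnected, so spawning has no cap.
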(event EventBeginPlay
  (Utilities|Time|SetTimerbyFunctionName 0 "DoSpawn" 3.0 true))

(event EventTick
  (params (DeltaSeconds :type Float%20%28single-precision%29)))

(fn DoSpawn
  (bind _randomlocation (Class|NavigationSystemV1|GetRandomLocationinNavigableRadius (Transformation|GetActorLocation (Components|GetOwner)) 1e+03 0 0))
  (bind _outrownames (DataTable|GetDataTableRowNames "/Game/HacknRush/Item/DT_Item.DT_Item"))
  (bind _returnvalue (Utilities|GetDataTableRow "/Game/HacknRush/Item/DT_Item.DT_Item" (.OutItem (Utilities|Array|Random _outrownames)))
    (:then
      (Game|SpawnActorfromClass (.ItemClass (Utilities|Struct|BreakST_Item _returnvalue)) (Math|Transform|MakeTransform _randomlocation "0, 0, 0" "1.000000,1.000000,1.000000") "Undefined" "MultiplyWithRoot" 0 0))))